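; Player parkour component that adds ledge hanging, climbing, crouching and foot IK to a Character.
; A 60 Hz looping timer drives foot placement plus gated hang and crouch updates.
; Jumping opens ledge detection, where traces find walkable ledges and pick the hang type, then MoveComponentTo snaps or climbs the capsule.
; Crouching interpolates speed and capsule height with trace-checked standing, while foot traces feed interpolated IK values.
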(event Custom|onMovementChanged
  (params (Prev%20Movement :type EMovementMode%20Enum :default "MOVE_None") (Current%20Movement :type EMovementMode%20Enum :default "MOVE_None"))
  ;[1 1 1] onMovementChanged
  (Utilities|IsValid (Variables|Default|GetCharacter%20Movement)
    (:Is%20Valid
      (Variables|Default|SetPrev%20Movement Prev%20Movement)
      (Variables|Default|SetCurrent%20Movement Current%20Movement))))

(event Custom|onUpdate
  ;[1 1 1] Tick
  (Utilities|FlowControl|Sequence
    (:then_0
      (|FootPlacement))
    (:then_1
      (|Hang))
    (:then_2
      (Character|Crouch))))

(event Custom|onClimbEnter
  ;[1 1 1] onClimbEnter
  (if (not (Variables|Hang|GetisClimbing?))
    (Variables|Hang|SetisHanging? false)
    (Variables|Hang|SetisClimbing? true)
    (Pawn|Components|CharacterMovement|SetMovementMode (Variables|Default|GetCharacter%20Movement) "MOVE_Flying" 0)
    (Components|Movement|StopMovementImmediately (Variables|Default|GetCharacter%20Movement))
    (Pawn|Components|CharacterMovement|DisableMovement (Variables|Default|GetCharacter%20Movement))
    (Variables|Default|SetCurrent%20Parkour%20Movement "NewEnumerator1")
    (Components|MoveComponentTo (Variables|Default|GetCapsule%20Component) (|TargetRelativeLocation_2) (|TargetRelativeRotation_2) true true 0.6 false)))

(event Custom|onClimbExit
  ;[1 1 1] onClimbExit
  (if (Variables|Hang|GetisClimbing?)
    (Variables|Default|SetCurrent%20Parkour%20Movement "NewEnumerator2")
    (Variables|Hang|SetisClimbing? false)
    (Variables|Hang|SetisHanging? false)
    (Components|MoveComponentTo (Variables|Default|GetCapsule%20Component) (|TargetRelativeLocation) (|TargetRelativeRotation) true true 0.2 false)
    (Utilities|FlowControl|Delay 0.05)
    (Pawn|Components|CharacterMovement|SetMovementMode (Variables|Default|GetCharacter%20Movement) "MOVE_Walking" 0)))

(event Custom|onHangExit
  ;[1 1 1] onHangExit
  (if (Variables|Hang|GetisHanging?)
    (Variables|Hang|SetisHanging? false)
    (Variables|Default|SetCurrent%20Parkour%20Movement "NewEnumerator2")
    (Pawn|Components|CharacterMovement|SetMovementMode (Variables|Default|GetCharacter%20Movement) "MOVE_Falling" 0)
    (CallFunction|CloseGates)
    (Utilities|Time|SetTimerbyFunctionName 0 "onOpenHangGate" 0.5)))

(event Custom|onHangEnter
  ;[1 1 1] onHangEnter
  (if (not (Variables|Hang|GetisHanging?))
    (Variables|Hang|SetisHanging? true)
    (Pawn|Components|CharacterMovement|SetMovementMode (Variables|Default|GetCharacter%20Movement) "MOVE_Flying" 0)
    (Components|Movement|StopMovementImmediately (Variables|Default|GetCharacter%20Movement))
    (Pawn|Components|CharacterMovement|DisableMovement (Variables|Default|GetCharacter%20Movement))
    (bind _hit (Hang|HangTypeTracer))
    (if _hit
      (Variables|Default|SetCurrent%20Parkour%20Movement "NewEnumerator0")
      (else
        (Variables|Default|SetCurrent%20Parkour%20Movement "NewEnumerator3")))
    (Components|MoveComponentTo (Variables|Default|GetCapsule%20Component) (|TargetRelativeLocation_Hang) (|TargetRelativeRotation_Hang) false false 0.13 false)))

(event Custom|onLand
  ;[1 1 1] OnLand
  (Jump|JumpEnd))

(event Custom|onJump
  ;[1 1 1] onJump
  (if (Utilities|CanJump?)
    (Jump|JumpStart)
    (else
      (Jump|JumpEvents))))

(event Custom|onCrouch
  (bind _current_parkour_movement (Variables|Default|GetCurrent%20Parkour%20Movement))
  ;[1 1 1] onCrouch
  (if (Math|Boolean|ORBoolean (Utilities|Enum|Equal(Enum) _current_parkour_movement "NewEnumerator2") (Utilities|Enum|Equal(Enum) _current_parkour_movement "NewEnumerator4") (Utilities|Enum|Equal(Enum) _current_parkour_movement "NewEnumerator5"))
    (if (Utilities|Enum|Equal(Enum) (Variables|Default|GetCurrent%20Parkour%20Movement) "NewEnumerator4")
      (Crouch|CrouchEnd)
      (else
        (Crouch|CrouchStart)))
    (else
      (Crouch|CrouchEvents))))

(event Custom|Initialize
  (params (Character :type Character%20Object%20Reference))
  ;[1 1 1] Initialize
  (|SetDefault Character)
  (Utilities|Time|SetTimerbyEvent (delegate Custom|onUpdate) 0.0167 true))

(fn HangUpdate
  (bind (_start _end) (Utilities|ForwardVectors))
  (bind (_start_2 _end_2) (Utilities|HeightVectors))
  (if (Utilities|CanHang?)
    (bind (_outhit _returnvalue) (Collision|LineTraceByChannel _start _end "TraceTypeQuery3" false 0 "None"))
    (if _returnvalue
      (Variables|Hang|SetWall%20Impact%20Point (.ImpactPoint (Collision|BreakHitResult _outhit)))
      (Variables|Hang|SetWall%20Impact%20Normal (.ImpactNormal (Collision|BreakHitResult _outhit)))
      (bind (_outhit_2 _returnvalue_2) (Collision|LineTraceByChannel _start_2 _end_2 "TraceTypeQuery3" false 0 "None"))
      (if _returnvalue_2
        (if (Class|CharacterMovementComponent|IsWalkable (Variables|Default|GetCharacter%20Movement) _outhit_2)
          (Variables|Hang|SetLedge%20Height%20Location (.ImpactPoint (Collision|BreakHitResult _outhit_2)))
          (if (|FarFromFloor?)
            (CallFunction|OnHangEnter)))))))

(fn HangTypeTracer
  (bind (_start _end) (Utilities|HangVectors))
  (bind _returnvalue (Collision|LineTraceByChannel _start _end "TraceTypeQuery3" false 0 "Persistent"))
  (return _returnvalue))

(fn HangJump
  (if (Utilities|Enum|Equal(Enum) (Variables|Default|GetCurrent%20Parkour%20Movement) "NewEnumerator0")
    (CallFunction|OnClimbEnter)))

(fn HangCrouch
  (bind _current_parkour_movement (Variables|Default|GetCurrent%20Parkour%20Movement))
  (if (or (Utilities|Enum|Equal(Enum) _current_parkour_movement "NewEnumerator0") (Utilities|Enum|Equal(Enum) _current_parkour_movement "NewEnumerator3"))
    (CallFunction|OnHangExit)))

(fn JumpStart
  (Character|Jump (Variables|Default|GetCharacter))
  (CallFunction|OpenGates))

(fn JumpEvents
  (Hang|HangJump)
  (Crouch|CrouchJump))

(fn JumpEnd
  (CallFunction|CloseGates))

(fn CrouchStart
  (Variables|Default|SetCurrent%20Parkour%20Movement "NewEnumerator4")
  (CallFunction|OnOpenCrouchGate))

(fn CrouchUpdate
  (bind _returnvalue (|getHalfHeight))
  (Variables|/Script/Engine.CharacterMovementComponent|SetMaxWalkSpeed (Variables|Default|GetCharacter%20Movement) (|getMaxWalkSpeed))
  (Components|Capsule|SetCapsuleHalfHeight (Variables|Default|GetCapsule%20Component) _returnvalue true)
  (Transformation|SetRelativeLocation (Variables|Default|GetMesh) (Math|Vector|MakeVector 0.0 0.0 (* _returnvalue -1.0)) false false))

(fn CrouchJump
  (bind _current_parkour_movement (Variables|Default|GetCurrent%20Parkour%20Movement))
  (if (or (Utilities|Enum|Equal(Enum) _current_parkour_movement "NewEnumerator4") (Utilities|Enum|Equal(Enum) _current_parkour_movement "NewEnumerator5"))
    (Crouch|CrouchEnd)))

(fn CrouchEvents
  (Hang|HangCrouch))

(fn CrouchEnd
  (bind (_start _end) (Utilities|UncrouchVectors))
  (bind _returnvalue (Collision|SphereTraceByChannel _start _end (Components|Capsule|GetScaledCapsuleRadius (Variables|Default|GetCapsule%20Component)) "TraceTypeQuery1" false 0 "ForOneFrame"))
  (if (not _returnvalue)
    (Variables|Default|SetCurrent%20Parkour%20Movement "NewEnumerator2")))

(fn OpenGates
  (CallFunction|OnOpenHangGate))

(fn CloseGates
  (CallFunction|OnCloseHangGate))

(fn FootPlacement
  (if (Utilities|CanFootPlace?)
    (bind (_blockinghit _distance) (Foot|FootDisplacement "foot_r"))
    (bind (_blockinghit_2 _distance_2) (Foot|FootDisplacement "foot_l"))
    (if (or _blockinghit_2 _blockinghit)
      (Variables|Foot|SetFoot%20Displacement (Math|Interpolation|FInterpTo (Variables|Foot|GetFoot%20Displacement) (* (- (Math|Float|SelectFloat _distance_2 _distance (>= _distance_2 _distance)) (Components|Capsule|GetScaledCapsuleHalfHeight (Variables|/Script/Engine.Character|GetCapsuleComponent (Variables|Default|GetCharacter)))) -1.0) (Utilities|Time|GetWorldDeltaSeconds) (Variables|Foot|GetIK%20Interp%20Speed)))
      (bind (_bblockinghit _distance_3 _normal) (Foot|FootRotation "foot_r"))
      (Variables|Foot|SetFoot%20R%20Rot (Math|Interpolation|RInterpTo (Variables|Foot|GetFoot%20R%20Rot) (Math|Rotator|MakeRotator (Class|KismetMathLibrary|DegAtan2 (.Y (Math|Vector|BreakVector _normal)) (.Z (Math|Vector|BreakVector _normal))) (* (Class|KismetMathLibrary|DegAtan2 (.X (Math|Vector|BreakVector _normal)) (.Z (Math|Vector|BreakVector _normal))) -1.0) 0.0) (Utilities|Time|GetWorldDeltaSeconds) (Variables|Foot|GetIK%20Interp%20Speed)))
      (Variables|Foot|SetR%20IK (Math|Interpolation|FInterpTo (Variables|Foot|GetR%20IK) (/ (- _distance_3 1.1e+02) -45.0) (Utilities|Time|GetWorldDeltaSeconds) (Variables|Foot|GetIK%20Interp%20Speed)))
      (bind (_bblockinghit_2 _distance_4 _normal_2) (Foot|FootRotation "foot_l"))
      (Variables|Foot|SetFoot%20L%20Rot (Math|Interpolation|RInterpTo (Variables|Foot|GetFoot%20L%20Rot) (Math|Rotator|MakeRotator (Class|KismetMathLibrary|DegAtan2 (.Y (Math|Vector|BreakVector _normal_2)) (.Z (Math|Vector|BreakVector _normal_2))) (* (Class|KismetMathLibrary|DegAtan2 (.X (Math|Vector|BreakVector _normal_2)) (.Z (Math|Vector|BreakVector _normal_2))) -1.0) 0.0) (Utilities|Time|GetWorldDeltaSeconds) (Variables|Foot|GetIK%20Interp%20Speed)))
      (Variables|Foot|SetL%20IK (Math|Interpolation|FInterpTo (Variables|Foot|GetL%20IK) (/ (- _distance_4 1.1e+02) -45.0) (Utilities|Time|GetWorldDeltaSeconds) (Variables|Foot|GetIK%20Interp%20Speed))))
    (else
      ;[1 1 1] Reset IK if you are not walking
      (Variables|Foot|SetFoot%20Displacement (Math|Interpolation|FInterpTo (Variables|Foot|GetFoot%20Displacement) 0.0 (Utilities|Time|GetWorldDeltaSeconds) (Variables|Foot|GetIK%20Interp%20Speed)))
      (Variables|Foot|SetFoot%20R%20Rot (Math|Interpolation|RInterpTo (Variables|Foot|GetFoot%20R%20Rot) "0, 0, 0" (Utilities|Time|GetWorldDeltaSeconds) (Variables|Foot|GetIK%20Interp%20Speed)))
      (Variables|Foot|SetR%20IK (Math|Interpolation|FInterpTo (Variables|Foot|GetR%20IK) 0.0 (Utilities|Time|GetWorldDeltaSeconds) (Variables|Foot|GetIK%20Interp%20Speed)))
      (Variables|Foot|SetFoot%20L%20Rot (Math|Interpolation|RInterpTo (Variables|Foot|GetFoot%20L%20Rot) "0, 0, 0" (Utilities|Time|GetWorldDeltaSeconds) (Variables|Foot|GetIK%20Interp%20Speed)))
      (Variables|Foot|SetL%20IK (Math|Interpolation|FInterpTo (Variables|Foot|GetL%20IK) 0.0 (Utilities|Time|GetWorldDeltaSeconds) (Variables|Foot|GetIK%20Interp%20Speed))))))

(fn FootDisplacement
  (params (InSocketName :type Name))
  (bind _character (Variables|Default|GetCharacter))
  (bind _character_2 (Variables|Default|GetCharacter))
  (bind _mesh (Variables|/Script/Engine.Character|GetMesh _character))
  (bind _capsulecomponent (Variables|/Script/Engine.Character|GetCapsuleComponent _character_2))
  (bind _returnvalue (Transformation|GetSocketLocation _mesh InSocketName))
  (bind _returnvalue_2 (Transformation|GetWorldLocation _mesh))
  (bind _returnvalue_3 (Components|Capsule|GetScaledCapsuleHalfHeight _capsulecomponent))
  (bind (_x _y) (Math|Vector|BreakVector _returnvalue))
  (bind _returnvalue_4 (+ _returnvalue_2 (Math|Vector|MakeVector 0.0 0.0 _returnvalue_3)))
  (bind _z (Math|Vector|BreakVector _returnvalue_4))
  (bind _returnvalue_5 (Math|Vector|MakeVector _x _y _z))
  (bind _outhit (Collision|LineTraceByChannel _returnvalue_5 (- _returnvalue_5 "0, 0,151.000000") "TraceTypeQuery1" false 0 "None"))
  (return (.bBlockingHit (Collision|BreakHitResult _outhit)) (.Distance (Collision|BreakHitResult _outhit))))

(fn FootRotation
  (params (InSocketName :type Name))
  (bind _character (Variables|Default|GetCharacter))
  (bind _mesh (Variables|/Script/Engine.Character|GetMesh _character))
  (bind _returnvalue (Transformation|GetSocketLocation _mesh "root"))
  (bind _returnvalue_2 (Transformation|GetSocketLocation _mesh InSocketName))
  (bind (_x _y) (Math|Vector|BreakVector _returnvalue_2))
  (bind _z (Math|Vector|BreakVector _returnvalue))
  (bind _returnvalue_3 (Math|Vector|MakeVector _x _y _z))
  (bind (_outhit _returnvalue_4) (Collision|LineTraceByChannel (+ _returnvalue_3 "0, 0,100.000000") (+ _returnvalue_3 "0, 0,-100.000000") "TraceTypeQuery1" false 0 "None"))
  (if _returnvalue_4
    (return (.bBlockingHit (Collision|BreakHitResult _outhit)) (.Distance (Collision|BreakHitResult _outhit)) (.Normal (Collision|BreakHitResult _outhit)))
    (else
      (return (.bBlockingHit (Collision|BreakHitResult _outhit)) 999.0 "0, 0, 0"))))

(event Custom|onOpenHangGate
  (Utilities|FlowControl|Gate true) ; enters at Open
)

(event Custom|onCloseHangGate
  (Utilities|FlowControl|Gate true) ; enters at Close
)

(event Custom|onOpenCrouchGate
  (Utilities|FlowControl|Gate true) ; enters at Open
)

(event Custom|onCloseCrouchGate
  (Utilities|FlowControl|Gate true) ; enters at Close
)